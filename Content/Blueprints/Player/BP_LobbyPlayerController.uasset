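; Player controller for the multiplayer lobby that manages the lobby menu, loading screen and session exit.
; On BeginPlay it sends the game instance's player name to the server and sets UI-only input for local controllers.
; Server events pass name and ready changes to BP_LobbyGameMode, while update events refresh player cards and ready status in the lobby widget.
; Ending the client session destroys it and opens the Menu level.
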(event `EndClientSession`
  (`DestroySessionCallbackProxy.DestroySession` self
    (:`then`
      (`GameplayStatics.OpenLevel` "Menu"))))

(event `CreateLoadingScreen`
  (`XRLoadingScreenFunctionLibrary.ShowLoadingScreen`))

(event `DestroyLoadingScreen`
  (bind _wpb_matchstart (`self.WPB_MatchStart`))
  (bind _foundwidgets (`WidgetBlueprintLibrary.GetAllWidgetsOfClass` "/Game/Blueprints/HUD/WBP_MatchStartWidget.WBP_MatchStartWidget_C"))
  (if (not (== (`KismetArrayLibrary.Array_Length` _foundwidgets) 0))
    (set `self.WPB_MatchStart` (`|GetArrayItem` _foundwidgets))
    (`/Engine/EditorBlueprintResources/StandardMacros.IsValid` _wpb_matchstart
      (:`Is Valid`
        (`/Game/Blueprints/HUD/WBP_MatchStartWidget.PlayTextClapsAnimation` _wpb_matchstart)
        (`Widget.RemoveFromParent` _wpb_matchstart)
        (`KismetSystemLibrary.PrintText` "Remove" true true (struct :`R` 1.0 :`G` 0.770315 :`A` 1.0) 8.0)))
    (else
      (`KismetSystemLibrary.PrintText` "Array 0" true true (struct :`R` 1.0 :`G` 0.770315 :`A` 1.0) 8.0))))

(event `DestroyLobbyMenu`
  (`Widget.RemoveFromParent` (`self.WB_LobbyMenu`)))

(event `CreateLobbyMenu`
  (`self.AddLobbyWidget`)
  (`WidgetBlueprintLibrary.SetInputMode_UIOnlyEx` self null)
  (set `self.bShowMouseCursor` true)
  (`self.UpdateLobbyWidget`))

(event `self.ReceiveBeginPlay`
  (bind _asbrackets_game_instance (cast `BracketsGameInstance` (`GameplayStatics.GetGameInstance`)))
  (bind _returnvalue (`BracketsGameInstance.GetPlayerName` _asbrackets_game_instance))
  (set `self.SteamID` _returnvalue)
  (`self.Server_UpdateSteamInfo` _returnvalue)
  (if (`self.IsLocalController`)
    (set `self.bShowMouseCursor` true)
    (`WidgetBlueprintLibrary.SetInputMode_UIOnlyEx` self null)))

(event `UpdatePlayerCard`
  (params (AllPlayerControllers :type "Array of /Game/Blueprints/Player/BP_LobbyPlayerController Object Reference") (SteamName :type "Array of Text"))
  (bind _wb_lobbymenu (`self.WB_LobbyMenu`))
  ;[1 1 1] UpdatePlayerNames
  (`/Engine/EditorBlueprintResources/StandardMacros.IsValid` _wb_lobbymenu
    (:`Is Valid`
      (`/Game/Blueprints/HUD/Menu/WBP_LobbyMenu.ClearPlayerNames` _wb_lobbymenu)
      (`/Game/Blueprints/HUD/Menu/WBP_LobbyMenu.UpdatePlayerNames` _wb_lobbymenu AllPlayerControllers SteamName))))

(event `Server_UpdateSteamInfo`
  (params (SteamID :type Text))
  (bind _returnvalue (`GameplayStatics.GetGameMode`))
  (set `self.SteamID` SteamID)
  (if (`GameplayStatics.ObjectIsA` _returnvalue "/Game/Blueprints/GameMode/BP_LobbyGameMode.BP_LobbyGameMode_C")
    (bind _asbp_lobby_game_mode (cast `/Game/Blueprints/GameMode/BP_LobbyGameMode` _returnvalue))
    (`/Game/Blueprints/GameMode/BP_LobbyGameMode.UpdateLobby` _asbp_lobby_game_mode true false)))

(event `UpdateReady`
  (params (AllPlayerControllers :type "Array of /Game/Blueprints/Player/BP_LobbyPlayerController Object Reference") (IsReadyArray :type "Array of Boolean"))
  (bind _wb_lobbymenu (`self.WB_LobbyMenu`))
  ;[1 1 1] UpdatePlayerNames
  (`/Engine/EditorBlueprintResources/StandardMacros.IsValid` _wb_lobbymenu
    (:`Is Valid`
      (`/Game/Blueprints/HUD/Menu/WBP_LobbyMenu.UpdateReadyStatus` _wb_lobbymenu AllPlayerControllers IsReadyArray))))

(event `Ready`
  (if (`self.bIsReady`)
    (`self.Server_Ready` false)
    (else
      (`self.Server_Ready` true))))

(event `Server_Ready`
  (params (bIsReady :type Boolean))
  (set `self.bIsReady` bIsReady)
  (`KismetSystemLibrary.PrintString` (`KismetStringLibrary.Conv_BoolToString` (`self.bIsReady`)) true true (struct :`R` 1.0 :`G` 0.006496 :`A` 1.0) 8.0)
  (bind _asbp_lobby_game_mode (cast `/Game/Blueprints/GameMode/BP_LobbyGameMode` (`GameplayStatics.GetGameMode`)))
  (`/Game/Blueprints/GameMode/BP_LobbyGameMode.Check Ready` _asbp_lobby_game_mode self bIsReady))

(fn `UpdateLobbyWidget`
  (bind _lobbywidget (`self.LobbyWidget`))
  (`/Engine/EditorBlueprintResources/StandardMacros.IsValid` _lobbywidget
    (:`Is Valid`
      (bind _aswbp_lobby_menu (cast `/Game/Blueprints/HUD/Menu/WBP_LobbyMenu` _lobbywidget))
      (set `self.WB_LobbyMenu` _aswbp_lobby_menu))))

(fn `UserConstructionScript`)