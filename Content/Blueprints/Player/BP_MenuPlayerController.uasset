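; Player controller for the menu and lobby, managing menu, customization and match-start loading widgets with UI-only mouse input.
; On BeginPlay it stores the player state name in the game instance and sends it to the server as SteamID, prompting the menu game mode to update names.
; Ready toggles go through the server to the lobby game mode's check.
; Lobby creation is marked temporary, and the server party update is a stub.
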(event `DestroyLoadingScreen`
  (bind _wpb_matchstart (`self.WPB_MatchStart`))
  (bind _foundwidgets (`WidgetBlueprintLibrary.GetAllWidgetsOfClass` "/Game/Blueprints/HUD/WBP_MatchStartWidget.WBP_MatchStartWidget_C"))
  (if (not (== (`KismetArrayLibrary.Array_Length` _foundwidgets) 0))
    (set `self.WPB_MatchStart` (`|GetArrayItem` _foundwidgets))
    (`/Engine/EditorBlueprintResources/StandardMacros.IsValid` _wpb_matchstart
      (:`Is Valid`
        (`/Game/Blueprints/HUD/WBP_MatchStartWidget.PlayTextClapsAnimation` _wpb_matchstart)
        (`Widget.RemoveFromParent` _wpb_matchstart)))))

(event `ShowCustomizeWidget`
  (bind _asmenu_hud (cast `MenuHUD` (`self.GetHUD`)))
  (bind _customizationwidget (`MenuHUD.CustomizationWidget` _asmenu_hud))
  (`/Engine/EditorBlueprintResources/StandardMacros.IsValid` _customizationwidget
    (:`Is Valid`
      (`Widget.SetVisibility` _customizationwidget "Visible"))
    (:`Is Not Valid`
      (bind _returnvalue (`|CreateWidget` "/Game/Blueprints/HUD/Menu/CustomizationMenu/WBP_CustomizationWidget.WBP_CustomizationWidget_C" self))
      (`UserWidget.AddToViewport` _returnvalue 0))))

(event `CreateLoadingScreen`
  (`self.ShowLoadingScreen`))

(event `ShowMainMenu`
  (bind _returnvalue (`|CreateWidget` "/Game/Blueprints/HUD/Menu/WBP_MainMenuWidget.WBP_MainMenuWidget_C" self))
  (bind _output_get (set `self.WBP_Main Menu Widget` _returnvalue))
  (`UserWidget.AddToViewport` _output_get 0))

(event `UpdateParty`
  (`self.Server_UpdateParty`))

(event `self.ReceiveBeginPlay`
  (bind _returnvalue (`KismetTextLibrary.Conv_StringToText` (`PlayerState.GetPlayerName` (`GameplayStatics.GetPlayerState` 0))))
  (bind _asbrackets_game_instance (cast `BracketsGameInstance` (`GameplayStatics.GetGameInstance`)))
  (`BracketsGameInstance.SetPlayerName` _asbrackets_game_instance _returnvalue)
  (set `self.SteamID` _returnvalue)
  (`self.UpdateSteamID`)
  (if (`self.IsLocalController`)
    (set `self.bShowMouseCursor` true)
    (`WidgetBlueprintLibrary.SetInputMode_UIOnlyEx` self null)))

(event `Server_UpdateParty`
  (cast `/Game/Blueprints/GameMode/BP_MenuGameMode` (`GameplayStatics.GetGameMode`)))

(event `RemoveMainMenuWidget`
  (`Widget.RemoveFromParent` (`self.WBP_Main Menu Widget`)))

(event `FindALobby`
  (bind _asbp_menu_game_mode (cast `/Game/Blueprints/GameMode/BP_MenuGameMode` (`GameplayStatics.GetGameMode`)))
  (`/Game/Blueprints/GameMode/BP_MenuGameMode.CreateLobby` _asbp_menu_game_mode))

(event `Ready`
  (if (`self.bIsReady`)
    (`self.Server_Ready` false)
    (else
      (`self.Server_Ready` true))))

(event `UpdateSteamID`
  (`self.Server_UpdateSteamID` (`self.SteamID`)))

(event `self.UpdatePlayerCardInformation`
  (`/Game/Blueprints/HUD/Menu/WBP_MainMenuWidget.UpdatePlayerCardNames` (`self.WBP_Main Menu Widget`) (`self.AllPlayerNames`) (`self.AllPlayerIcons`) (`self.AllPlayerCards`)))

(event `Server_UpdateSteamID`
  (params (SteamID :type Text))
  (set `self.SteamID` SteamID)
  (bind _asbp_menu_game_mode (cast `/Game/Blueprints/GameMode/BP_MenuGameMode` (`GameplayStatics.GetGameMode`)))
  (`/Game/Blueprints/GameMode/BP_MenuGameMode.UpdateSteamNames` _asbp_menu_game_mode))

(event `Server_Ready`
  (params (bIsReady :type Boolean))
  (set `self.bIsReady` bIsReady)
  (`KismetSystemLibrary.PrintString` (`KismetStringLibrary.Conv_BoolToString` (`self.bIsReady`)) true true (struct :`R` 1.0 :`G` 0.006496 :`A` 1.0) 8.0)
  (bind _asbp_lobby_game_mode (cast `/Game/Blueprints/GameMode/BP_LobbyGameMode` (`GameplayStatics.GetGameMode`)))
  (`/Game/Blueprints/GameMode/BP_LobbyGameMode.Check Ready` _asbp_lobby_game_mode null bIsReady))

(fn `ShowLoadingScreen`
  (`/Engine/EditorBlueprintResources/StandardMacros.IsValid` (`self.WPB_MatchStart`)
    (:`Is Valid`
      _)
    (:`Is Not Valid`
      (bind _returnvalue (`|CreateWidget` "/Game/Blueprints/HUD/WBP_MatchStartWidget.WBP_MatchStartWidget_C" (`GameplayStatics.GetPlayerControllerFromID` 0)))
      (set `self.WPB_MatchStart` _returnvalue)))
  (`UserWidget.AddToViewport` (`self.WPB_MatchStart`) 0))

(fn `UpdateColorButtons`
  (params (NewParam :type "/Game/Blueprints/HUD/Menu/CustomizationMenu/WBP_ColorButton Object Reference"))
  (`/Game/Blueprints/HUD/Menu/CustomizationMenu/WBP_CustomizationWidget.UpdateColorButtons` (`/Game/Blueprints/HUD/Menu/WBP_MainMenuWidget.WBP_CustomizationWidget` (`self.WBP_Main Menu Widget`)) NewParam))

(fn `UserConstructionScript`)