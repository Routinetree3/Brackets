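; BP_BracketsPlayerController is a player controller offering a few custom events for view rotation, loading screen removal and camera shake.
; RotatePlayer sets the control rotation to a given yaw with zero pitch and roll, and StartCameraShake starts the base weapon shake.
; DIsableLoadingScreen calls HideLoadingScreen, which finds the first top-level WBP_MatchStartWidget, starts its text claps animation and immediately removes it, printing debug text.
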(event `RotatePlayer`
  (params (`New Rotation Z (Yaw)` :type "Float (single-precision)"))
  (`self.SetControlRotation` (`KismetMathLibrary.MakeRotator` 0.0 0.0 `New Rotation Z (Yaw)`)))

(event `DIsableLoadingScreen`
  (`self.HideLoadingScreen`))

(event `self.StartCameraShake`
  (`self.ClientStartCameraShake` "/Game/Blueprints/Weapons/CameraShake/BaseWeapon_CameraShake.BaseWeapon_CameraShake_C"))

(fn `HideLoadingScreen`
  (bind _wbp_matchstartwidget (`self.WBP_MatchStartWidget`))
  (bind _foundwidgets (`WidgetBlueprintLibrary.GetAllWidgetsOfClass` "/Game/Blueprints/HUD/WBP_MatchStartWidget.WBP_MatchStartWidget_C"))
  (if (not (== (`KismetArrayLibrary.Array_Length` _foundwidgets) 0))
    (set `self.WBP_MatchStartWidget` (`|GetArrayItem` _foundwidgets))
    (`/Engine/EditorBlueprintResources/StandardMacros.IsValid` (`self.WBP_MatchStartWidget`)
      (:`Is Valid`
        (`/Game/Blueprints/HUD/WBP_MatchStartWidget.PlayTextClapsAnimation` _wbp_matchstartwidget)
        (`Widget.RemoveFromParent` _wbp_matchstartwidget)
        (`KismetSystemLibrary.PrintText` "Remove" true true (struct :`R` 1.0 :`G` 0.770315 :`A` 1.0) 8.0)))
    (else
      (`KismetSystemLibrary.PrintText` "Array 0" true true (struct :`R` 1.0 :`G` 0.770315 :`A` 1.0) 8.0))))

(fn `UserConstructionScript`)