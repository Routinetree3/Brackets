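; Lobby game mode that tracks connected players and their ready states, then moves them out of the lobby into a match or ends their sessions.
; Join and logout update parallel controller and ready arrays, and UpdateLobby pushes Steam-name cards or ready states to every controller.
; CheckReady recounts ready players.
; AllPlayerReadyforGame shows loading screens and travels to the match, while ReadyCountdownFinished ends client sessions, host last after a short delay.
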(event `self.ReceiveBeginPlay`)

(event `Check Ready`
  (params (PlayerController :type "/Game/Blueprints/Player/BP_LobbyPlayerController Object Reference") (IsReady :type Boolean))
  (set `self.NumberOfPlayersReady` 0)
  (`KismetArrayLibrary.Array_Set` (`self.IsReadyArray`) (`KismetArrayLibrary.Array_Find` (`self.AllConnectedPlayers`) PlayerController) IsReady true)
  (`self.UpdateLobby` false true)
  (for _array_element (`self.IsReadyArray`)
    (if _array_element
      (`/Engine/EditorBlueprintResources/StandardMacros.IncrementInt` (`self.NumberOfPlayersReady`)
        (:`  `
          _)))
    (`self.UpdateLobby` false true)))

(event `self.ReadyCountdownFinished`
  (bind _allconnectedplayers (`self.AllConnectedPlayers`))
  (for _array_element _allconnectedplayers
    (`/Game/Blueprints/Player/BP_LobbyPlayerController.CreateLoadingScreen` _array_element)
    (`/Game/Blueprints/Player/BP_LobbyPlayerController.DestroyLobbyMenu` _array_element)
    (if (!= _array_element (`GameplayStatics.GetPlayerController` 0))
      (`/Game/Blueprints/Player/BP_LobbyPlayerController.EndClientSession` _array_element)))
  (`KismetSystemLibrary.Delay` 0.2)
  (`/Game/Blueprints/Player/BP_LobbyPlayerController.EndClientSession` (`|GetArrayItem` _allconnectedplayers)))

(event `self.HandleStartingNewPlayer`
  (params (NewPlayer :type "PlayerController Object Reference"))
  (bind _asbp_lobby_player_controller (cast `/Game/Blueprints/Player/BP_LobbyPlayerController` NewPlayer))
  (bind _returnvalue (`KismetArrayLibrary.Array_Add` (`self.AllConnectedPlayers`) _asbp_lobby_player_controller))
  (`KismetArrayLibrary.Array_Set` (`self.IsReadyArray`) _returnvalue false true)
  (`/Engine/EditorBlueprintResources/StandardMacros.IsValid` (`LobbyPlayerController.LobbyWidget` _asbp_lobby_player_controller)
    (:`Is Valid`
      _)
    (:`Is Not Valid`
      (`/Game/Blueprints/Player/BP_LobbyPlayerController.CreateLobbyMenu` _asbp_lobby_player_controller)))
  (`self.UpdateLobby` true)
  (`/Game/Blueprints/Player/BP_LobbyPlayerController.DestroyLoadingScreen` _asbp_lobby_player_controller))

(event `self.AllPlayerReadyForGame`
  (for _array_element (`self.AllConnectedPlayers`)
    (`/Game/Blueprints/Player/BP_LobbyPlayerController.CreateLoadingScreen` _array_element)
    (`/Game/Blueprints/Player/BP_LobbyPlayerController.DestroyLobbyMenu` _array_element))
  (`self.TravelToGame` (`self.MatchLevelLocation`)))

(event `self.K2_OnLogout`
  (params (ExitingController :type "Controller Object Reference"))
  (bind _allconnectedplayers (`self.AllConnectedPlayers`))
  (bind _asbp_lobby_player_controller (cast `/Game/Blueprints/Player/BP_LobbyPlayerController` ExitingController))
  (bind _returnvalue (`KismetArrayLibrary.Array_Find` _allconnectedplayers _asbp_lobby_player_controller))
  (`KismetArrayLibrary.Array_Remove` (`self.IsReadyArray`) _returnvalue)
  (`KismetArrayLibrary.Array_Remove` _allconnectedplayers _returnvalue)
  (`self.UpdateLobby` true))

(event `UpdateLobby`
  (params (PlayerCard :type Boolean) (ReadyStae :type Boolean))
  (bind _allconnectedplayers (`self.AllConnectedPlayers`))
  (bind _allconnectedplayers_2 (`self.AllConnectedPlayers`))
  (if PlayerCard
    (`KismetArrayLibrary.Array_Clear` (`self.AllAvatarArray`))
    (`KismetArrayLibrary.Array_Clear` (`self.SteamNamesArray`))
    (for _array_element _allconnectedplayers_2
      (`KismetArrayLibrary.Array_Add` (`self.SteamNamesArray`) (`/Game/Blueprints/Player/BP_LobbyPlayerController.SteamID` _array_element)))
    (for _array_element_2 _allconnectedplayers_2
      (`/Game/Blueprints/Player/BP_LobbyPlayerController.UpdatePlayerCard` _array_element_2 _allconnectedplayers_2 (`self.SteamNamesArray`)))
    (elif ReadyStae
      (for _array_element_3 _allconnectedplayers
        (`/Game/Blueprints/Player/BP_LobbyPlayerController.UpdateReady` _array_element_3 _allconnectedplayers (`self.IsReadyArray`))))))

(fn `UserConstructionScript`)