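; Main menu game mode that brings joining players into the menu and hosts lobbies through Advanced Sessions.
; New players get a timed loading screen before the main menu, and their controllers are tracked to rebuild a Steam ID list.
; BeginPlay opens a small friends-only presence session, while CreateLobby creates a larger one and travels to the Lobby as listen server.
; Beacon events handle host success and record connecting clients; an unconnected find-or-join branch never runs.
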(event `CreateLobby`
  (bind _asbp_menu_player_controller (cast `/Game/Blueprints/Player/BP_MenuPlayerController` (`GameplayStatics.GetPlayerController` 0)))
  (`/Game/Blueprints/Player/BP_MenuPlayerController.CreateLoadingScreen` _asbp_menu_player_controller)
  (`/Game/Blueprints/Player/BP_MenuPlayerController.RemoveMainMenuWidget` _asbp_menu_player_controller)
  (`CreateSessionCallbackProxyAdvanced.CreateAdvancedSession` :`PlayerController` _asbp_menu_player_controller :`PublicConnections` 32
    (:`OnSuccess`
      (`AdvancedSessionsLibrary.ServerTravel` "/Game/Levels/Lobby?listen" true))))

(event `self.ReceiveBeginPlay`
  (`CreateSessionCallbackProxyAdvanced.CreateAdvancedSession` :`PlayerController` (`GameplayStatics.GetPlayerController` 0) :`PublicConnections` 5 :`bAllowJoinViaPresence` false :`bAllowJoinViaPresenceFriendsOnly` true))

(event `self.HandleStartingNewPlayer`
  (params (NewPlayer :type "PlayerController Object Reference"))
  (bind _asbp_menu_player_controller (cast `/Game/Blueprints/Player/BP_MenuPlayerController` NewPlayer))
  (`KismetArrayLibrary.Array_Add` (`self.AllControllers`) _asbp_menu_player_controller)
  (`/Game/Blueprints/Player/BP_MenuPlayerController.ShowLoadingScreen` _asbp_menu_player_controller)
  (`KismetSystemLibrary.Delay` 5.0)
  (`/Game/Blueprints/Player/BP_MenuPlayerController.ShowMainMenu` _asbp_menu_player_controller)
  (`/Game/Blueprints/Player/BP_MenuPlayerController.DestroyLoadingScreen` _asbp_menu_player_controller))

(event `UpdateSteamNames`
  (`KismetArrayLibrary.Array_Clear` (`self.SteamID`))
  (for _array_element (`self.AllControllers`)
    (`KismetArrayLibrary.Array_Add` (`self.SteamID`) (`/Game/Blueprints/Player/BP_MenuPlayerController.SteamID` _array_element))))

(event `self.UpdateNewPlayerInformation`
  (params (NewClientActor :type "OnlineBeaconClient Object Reference"))
  (bind _asbrackets_beacon_client (cast `BracketsBeaconClient` NewClientActor))
  (bind _returnvalue (`KismetArrayLibrary.Array_Add` (`self.Client Actor Array`) _asbrackets_beacon_client))
  (`KismetSystemLibrary.PrintString` (`KismetStringLibrary.Conv_IntToString` _returnvalue)))

(event `BP_OnHostSuccess`
  (bind _returnvalue (`GameplayStatics.GetCurrentLevelName` true))
  (`self.OnHostSuccess` _returnvalue)
  (`self.On host set`))

(fn `UserConstructionScript`)