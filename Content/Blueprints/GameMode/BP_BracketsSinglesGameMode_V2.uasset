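; Game mode for a singles bracket match that places players at player starts as the match and its rounds progress.
; On InProgress it polls on a delay until the controller count reaches the player limit, then moves players to numbered starts, clears loading screens and initializes the match.
; After each round ends, a delayed pass sends dead players to the default start and packs survivors into sequential numbered starts using a counter that then resets.
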(event `self.K2_OnSetMatchState`
  (params (NewState :type Name))
  (bind _bpconrrollerarray (`self.BPConrrollerArray`))
  (if (== "InProgress" NewState)
    (`KismetSystemLibrary.Delay` 2.0 :!label _label)
    (`self.BackUpCheck`
      (:`then`
        (for (_ _array_index) (`self.ControllerArray`)
          (`self.MakeBPArray` _array_index))
        (`self.InitilizeLocation`)
        (`self.HandleMatchInitilization`)
        (`KismetSystemLibrary.PrintText` "Initilized"))
      (:`then2`
        (goto _label)))
    (else
      (if (== NewState "RoundStart")
        (`KismetSystemLibrary.PrintText` "RoundStart" true true (struct :`G` 0.66 :`B` 1.0 :`A` 1.0) 15.0))
      (if (== NewState "RoundInProgress")
        (`KismetSystemLibrary.PrintText` "InProgress" true true (struct :`R` 1.0 :`B` 0.124342 :`A` 1.0) 10.0))
      (if (== NewState "RoundEnd")
        (`KismetSystemLibrary.Delay` 2.0)
        (for (_ _array_index_2) _bpconrrollerarray
          (`self.ProgressPlayerLocation` _bpconrrollerarray _array_index_2))
        (set `self.SpawnStartItteration` 0)))))

(event `self.ReceiveBeginPlay`)

(fn `AddSpawnStartItteration`
  (set `self.SpawnStartItteration` (+ (`self.SpawnStartItteration`) 1)))

(fn `Check if Dead`
  (params (`Controller Array` :type "Array of /Game/Blueprints/Player/BP_BracketsPlayerController Object Reference (by ref)") (`Array Index` :type Integer))
  (returns (bIsDead :type Boolean) (ControllerCheacked :type "/Game/Blueprints/Player/BP_BracketsPlayerController Object Reference"))
  (bind _output (`|GetArrayItem` `Controller Array` `Array Index`))
  (bind _asbrackets_player_state (cast `BracketsPlayerState` (`Controller.PlayerState` _output)))
  (return (`BracketsPlayerState.bIsDead` _asbrackets_player_state) _output))

(fn `ChoosePlayerStart`
  (params (Player :type "Controller Object Reference"))
  (returns (ReturnValue :type "Actor Object Reference"))
  (return (`self.K2_FindPlayerStart` Player "Default")))

(fn `UserConstructionScript`
  (bind _outactors (`GameplayStatics.GetAllActorsOfClass` "/Script/Engine.PlayerStart"))
  (bind _output_get (set `self.PlayerStartArray` _outactors)))